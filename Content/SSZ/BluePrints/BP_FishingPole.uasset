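; BP_FishingPole is a fishing pole actor that spawns and tethers a physics-constrained lure when play begins.
; On BeginPlay it spawns a scaled-down BP_Lure slightly offset from and below the pole, then attaches the Cable's end to it.
; The cable length is set to a fraction of the pole-to-lure distance, and a PhysicsConstraint links the pole's Cylinder to the lure's Lure component.
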(event EventBeginPlay
  (bind _returnvalue (Transformation|GetActorLocation))
  (bind _cable (Variables|Default|GetCable))
  (bind _returnvalue_2 (Game|SpawnActorfromClass "/Game/SSZ/BluePrints/BP_Lure.BP_Lure_C" (Math|Transform|MakeTransform (Math|Vector|MakeVector (+ (.x _returnvalue) 25.0) (.y _returnvalue) (- (.z _returnvalue) 3e+01)) "0, 0, 0" "0.100000,0.100000,0.100000") "AlwaysSpawn" 0 0))
  (Class|CableComponent|SetAttachEndto _cable _returnvalue_2 "None" "None")
  (Variables|/Script/CableComponent.CableComponent|SetCableLength _cable (* (CallFunction|DistanceBetweenVectors (Transformation|GetActorLocation _returnvalue_2) (Transformation|GetActorLocation)) 0.1))
  (Class|PhysicsConstraintComponent|SetConstrainedComponents (Variables|Default|GetPhysicsConstraint) (Variables|Default|GetCylinder) "None" (Variables|/Game/SSZ/BluePrints/BP_Lure.BP_Lure_C|GetLure _returnvalue_2) "None"))

(fn ConstructionScript)