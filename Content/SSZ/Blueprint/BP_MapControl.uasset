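; BP_MapControl loads and swaps a map at runtime as a streamed level instance.
; LoadLevel spawns MapToLoad at the world origin and stores the instance in LoadedLevelRef.
; If a level is already loaded, it calls UnloadLevel, waits a zero-second delay, then calls itself again.
; UnloadLevel clears the instance's ShouldBeLoaded flag and empties the reference.
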(event Custom|LoadLevel
  ;[1 1 1] Check if level is loaded
  (Utilities|IsValid (Variables|GameplayControls|GetLoadedLevelRef)
    (:Is%20Valid
      ;[1 1 1] If Yes then unload previous map then trigger load sequence again
      (CallFunction|UnloadLevel)
      (Utilities|FlowControl|Delay 0.0)
      (CallFunction|LoadLevel))
    (:Is%20Not%20Valid
      ;[1 1 1] Load Level and set refrence to it for later
      (bind _returnvalue (Class|LevelStreamingDynamic|LoadLevelInstance (Variables|UserSettings|GetMapToLoad) "0, 0, 0" "0, 0, 0"))
      (Variables|GameplayControls|SetLoadedLevelRef _returnvalue))))

(event Custom|UnloadLevel
  ;[1 1 1] Unloads the currently loaded level and clears level refrence
  (Variables|/Script/Engine.LevelStreaming|SetbShouldBeLoaded (Variables|GameplayControls|GetLoadedLevelRef) false)
  (Variables|GameplayControls|SetLoadedLevelRef 0))

(fn ConstructionScript)