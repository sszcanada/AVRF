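; Level settings actor that applies per-level AVRF configuration: info data, controls, UI and VR hand controllers.
; On BeginPlay, after a short delay, it pushes its assets to the main game mode and info levels, then calls SwitchControllers on the BP_Pawn_VR.
; ChangeController reapplies controls, UI and controllers at runtime from its variables.
; EasyContollerSwitch does the same with caller-supplied values for use from other Blueprints.
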(event Custom|ChangeController
  (bind _self self)
  ;[1 1 1] Change Your Controllers and Info At Runtime
  (bind _infolevels (CallFunction|GetInfoLevels _self))
  (Variables|/Game/AVRFramework/Blueprints/Info/BP_Info_Level.BP_Info_Level_C|SetInfoControls _infolevels (Variables|LevelSettings|GetInfoControlsToUse))
  (bind _asbp_game_mode_main (CallFunction|GetMainGameMode _self))
  (Default|UpdateInfoControls _asbp_game_mode_main)
  (Variables|/Game/AVRFramework/Blueprints/Info/BP_Info_Level.BP_Info_Level_C|SetInfoUI _infolevels (Variables|LevelSettings|GetInfoUIToUse))
  (Default|UpdateInfoUI _asbp_game_mode_main)
  (bind _player_controller (CallFunction|GetMainPlayerController _self))
  (bind _asbp_pawn_vr (Utilities|Casting|CastToBP_Pawn_VR (Pawn|GetControlledPawn _player_controller)))
  (CallFunction|GetInfoControls self)
  (Default|SwitchControllers _asbp_pawn_vr (Variables|ControllerSettings|GetLeftControllerToUse) (Variables|ControllerSettings|GetRightControllerToUse)))

(event Custom|EasyContollerSwitch
  (params (InfoControlsToUse :type BP%20Info%20Controls%20Class%20Reference) (InfoUIToUse :type BP%20Info%20UI%20Class%20Reference) (LeftControllerToUse :type BP%20Base%20Motion%20Controller%20Class%20Reference) (RightControllerToUse :type BP%20Base%20Motion%20Controller%20Class%20Reference))
  (bind _self self)
  ;[1 1 1] Event to easily change the controls from another blueprint
  (bind _infolevels (CallFunction|GetInfoLevels _self))
  (Variables|/Game/AVRFramework/Blueprints/Info/BP_Info_Level.BP_Info_Level_C|SetInfoControls _infolevels InfoControlsToUse)
  (bind _asbp_game_mode_main (CallFunction|GetMainGameMode _self))
  (Default|UpdateInfoControls _asbp_game_mode_main)
  (Variables|/Game/AVRFramework/Blueprints/Info/BP_Info_Level.BP_Info_Level_C|SetInfoUI _infolevels InfoUIToUse)
  (Default|UpdateInfoUI _asbp_game_mode_main)
  (bind _player_controller (CallFunction|GetMainPlayerController _self))
  (bind _asbp_pawn_vr (Utilities|Casting|CastToBP_Pawn_VR (Pawn|GetControlledPawn _player_controller)))
  (CallFunction|GetInfoControls self)
  (Default|SwitchControllers _asbp_pawn_vr LeftControllerToUse RightControllerToUse))

(event EventBeginPlay
  (bind _self self)
  ;[1 1 1] Setup AVRF files to run you levels
  (Utilities|FlowControl|Delay 1.0)
  (bind _asbp_game_mode_main (CallFunction|GetMainGameMode _self))
  (Variables|/Game/AVRFramework/Framework/BP_GameMode_Main.BP_GameMode_Main_C|SetDefaultInfoData _asbp_game_mode_main (Variables|LevelSettings|GetInfoDataToUse))
  (Default|UpdateInfoData _asbp_game_mode_main)
  (bind _infolevels (CallFunction|GetInfoLevels _self))
  (Variables|/Game/AVRFramework/Blueprints/Info/BP_Info_Level.BP_Info_Level_C|SetInfoControls _infolevels (Variables|LevelSettings|GetInfoControlsToUse))
  (Default|UpdateInfoControls _asbp_game_mode_main)
  (Variables|/Game/AVRFramework/Blueprints/Info/BP_Info_Level.BP_Info_Level_C|SetInfoUI _infolevels (Variables|LevelSettings|GetInfoUIToUse))
  (Default|UpdateInfoUI _asbp_game_mode_main)
  (bind _player_controller (CallFunction|GetMainPlayerController _self))
  (bind _asbp_pawn_vr (Utilities|Casting|CastToBP_Pawn_VR (Pawn|GetControlledPawn _player_controller)))
  (CallFunction|GetInfoControls self)
  (Default|SwitchControllers _asbp_pawn_vr (Variables|ControllerSettings|GetLeftControllerToUse) (Variables|ControllerSettings|GetRightControllerToUse)))

(fn ConstructionScript)